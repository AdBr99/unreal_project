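; Planet actor that orbits around a center location at a set angular speed.
; Each Tick, OrthogonalizeAxis uses a double cross product to make the orbit axis a unit vector perpendicular to the current radius.
; The center-to-actor offset is then rotated around that axis by Speed times delta time to set the new location.
; Debug lines for the radius and axis exist but are not connected.
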(event `orthogonalize axis`
  (bind _returnvalue (- (`self.K2_GetActorLocation`) (`self.CenterLocation`)))
  (set `self.Axis` (`KismetMathLibrary.Normal` (`KismetMathLibrary.Cross_VectorVector` _returnvalue (`KismetMathLibrary.Cross_VectorVector` (`self.Axis`) _returnvalue)))))

(event `self.ReceiveTick`
  (params (DeltaSeconds :type "Float (single-precision)"))
  (`self.orthogonalize axis`)
  (`self.K2_SetActorLocation` (+ (`KismetMathLibrary.RotateAngleAxis` (- (`self.K2_GetActorLocation`) (`self.CenterLocation`)) (* DeltaSeconds (`self.Speed`)) (`self.Axis`)) (`self.CenterLocation`))))

(fn `UserConstructionScript`)